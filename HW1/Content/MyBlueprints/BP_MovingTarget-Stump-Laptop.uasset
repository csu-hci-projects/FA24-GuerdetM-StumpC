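; BP_MovingTarget-Stump-Laptop is a shootable target actor that takes damage from player projectiles and reports its destruction to the player character.
; Health starts at MaxHealth on BeginPlay and drops by a fixed amount on each BP_FirstPersonProjectile hit.
; At zero health it increments TargetsHit on BP_FirstPersonCharacter, calls CheckTargets, then destroys itself.
; Despite its name, this Blueprint's graphs contain no movement logic.
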(event EventBeginPlay
  (Variables|Default|SetCurrentHealth (Variables|Default|GetMaxHealth)))

(event Collision|EventHit
  (params (MyComp :type Primitive%20Component%20Object%20Reference) (Other :type Actor%20Object%20Reference) (OtherComp :type Primitive%20Component%20Object%20Reference) (bSelfMoved :type Boolean) (HitLocation :type Vector :default "0, 0, 0") (HitNormal :type Vector :default "0, 0, 0") (NormalImpulse :type Vector :default "0, 0, 0") (Hit :type Hit%20Result%20Structure%20%28by%20ref%29))
  (Utilities|Casting|CastToBP_FirstPersonProjectile Other)
  (bind _asbp_first_person_character (Utilities|Casting|CastToBP_FirstPersonCharacter (Game|GetPlayerCharacter 0)))
  (Variables|Default|SetCurrentHealth (- (Variables|Default|GetCurrentHealth) 2e+01))
  (if (<= (Variables|Default|GetCurrentHealth) 0.0)
    (Variables|/Game/FirstPerson/Blueprints/BP_FirstPersonCharacter.BP_FirstPersonCharacter_C|SetTargetsHit _asbp_first_person_character (+ (Variables|/Game/FirstPerson/Blueprints/BP_FirstPersonCharacter.BP_FirstPersonCharacter_C|GetTargetsHit _asbp_first_person_character) 1))
    (Default|CheckTargets _asbp_first_person_character)
    (Actor|DestroyActor)))

(fn ConstructionScript)